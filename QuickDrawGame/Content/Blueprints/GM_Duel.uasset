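; GM_Duel runs the timing of a quick-draw duel, moving the round through Intro, Wait and Draw phases.
; On BeginPlay it finds and stores the level's BP_Alert actor.
; Tick accumulates time during Intro, then switches to Wait and starts a random delay within the configured draw bounds.
; When the delay ends it enters Draw and makes the alert visible, printing a message if the reference is invalid.
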(event `self.ReceiveBeginPlay`
  (bind _returnvalue (`GameplayStatics.GetActorOfClass` "/Game/Blueprints/BP_Alert.BP_Alert_C"))
  (set `self.Alert Reference` _returnvalue))

(event `self.ReceiveTick`
  (params (DeltaSeconds :type "Float (single-precision)"))
  (switch `/Game/Blueprints/Enums/E_Phase` (`self.Phase`)
    (:`NewEnumerator0`
      (set `self.ElapsedTime` (+ DeltaSeconds (`self.ElapsedTime`)))
      (if (>= (`self.ElapsedTime`) (`self.RoundStartTime`))
        (set `self.Phase` "NewEnumerator1")
        (`KismetSystemLibrary.Delay` (`KismetMathLibrary.RandomFloatInRange` (`self.MinDrawDelay`) (`self.MaxDrawDelay`)))
        (set `self.Phase` "NewEnumerator2")
        (`/Engine/EditorBlueprintResources/StandardMacros.IsValid` (`self.Alert Reference`)
          (:`Is Valid`
            (`/Game/Blueprints/BP_Alert.SetVisibility` (`self.Alert Reference`) true))
          (:`Is Not Valid`
            (`KismetSystemLibrary.PrintString` "Alert Not FOUND")))))))

(fn `UserConstructionScript`)