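; Samurai duelist for the GM_Duel game mode, a paper sprite that slides into position and responds to a draw input.
; On BeginPlay it caches the game mode, hides the Cross marker and runs a double-speed timeline that lerps the sprite from its slide start to its default position.
; Attack handles only the Wait phase, where a draw shows the Cross and sets PressedDraw to block further attempts.
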(event `self.ReceiveBeginPlay`
  (bind _asgm_duel (cast `/Game/Blueprints/GM_Duel` (`GameplayStatics.GetGameMode`)))
  (set `self.GameMode` _asgm_duel)
  (set `self.SpriteDefaultPosition` (`SceneComponent.RelativeLocation` (`self.PaperSprite`)))
  (`self.SlideIn`)
  (`self.Set Cross Visibility` false))

(event `SlideIn`
  (`TimelineComponent.SetPlayRate` (`self.SlideInAnimate`) 2.0)
  (bind (_direction _alpha) (`Timeline|SlideInAnimate` :!via `PlayFromStart`)
    (:`Update`
      (`SceneComponent.K2_SetRelativeLocation` (`self.PaperSprite`) (`KismetMathLibrary.VLerp` (`self.Slide Start Position`) (`self.SpriteDefaultPosition`) _alpha) false false))))

(event `Attack`
  (if (not (`self.PressedDraw`))
    (switch `/Game/Blueprints/Enums/E_Phase` (`/Game/Blueprints/GM_Duel.Phase` (`self.GameMode`))
      (:`NewEnumerator1`
        (`self.Set Cross Visibility` true)
        (set `self.PressedDraw` true)))))

(fn `Set Cross Visibility`
  (params (bNewVisibility :type Boolean))
  (`SceneComponent.SetVisibility` (`self.Cross`) bNewVisibility false))

(fn `UserConstructionScript`)